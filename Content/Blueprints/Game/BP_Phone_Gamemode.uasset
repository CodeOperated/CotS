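; Game mode Blueprint, named for a phone mode, that starts a sound and shows a background HUD when play begins.
; BeginPlay plays a 2D sound, then creates the HUD_Background widget, stores it and adds it to the viewport.
; GetBGInfo looks up a background type and image in DT_Background using a row number as the row name.
; Background switching is unfinished: SwitchToBG is empty, and neither function runs from the event graph.
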(event EventBeginPlay
  (Audio|SpawnSound2D "/Game/Music/wip_norm__1_.wip_norm__1_" 1.0 1.0 0.0 0)
  (bind _returnvalue (UserInterface|CreateWidget "/Game/Blueprints/HUD/HUD_Background.HUD_Background_C"))
  (bind _output_get (Variables|Default|SetHUD_BG_Ref _returnvalue))
  (UserInterface|Viewport|AddtoViewport _output_get 0))

(fn ConstructionScript)

(fn SwitchtoBG)

(fn GetBGInfo
  (bind _returnvalue (Utilities|GetDataTableRow "/Game/DataTables/DT_Background.DT_Background" (Utilities|String|StringToName (Utilities|String|ToString(Integer) (Variables|Default|GetrowNumber))))
    (:then
      (return (.E_Background (Utilities|Struct|BreakS_Background _returnvalue)) (.BackgroundImage (Utilities|Struct|BreakS_Background _returnvalue))))))